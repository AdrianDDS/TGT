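; Actor that moves a skeletal mesh along its spline component at a rate set by Speed.
; Each Tick adds Speed times delta time to Distance, then snaps the mesh to the spline's world location and rotation there.
; A fixed -90 degree rotation offset follows, and Distance has no looping or clamping.
; Unconnected leftovers hold a length-fraction version of the movement and attempts to read the character's velocity.
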(event `self.ReceiveBeginPlay`)

(event `self.ReceiveTick`
  (params (DeltaSeconds :type "Float (single-precision)"))
  (set `self.Distance` (+ (* DeltaSeconds (`self.Speed`)) (`self.Distance`)))
  (`SceneComponent.K2_SetWorldTransform` (`self.SkeletalMesh`) (`KismetMathLibrary.MakeTransform` (`SplineComponent.GetLocationAtDistanceAlongSpline` (`self.Spline`) (`self.Distance`) "World") (`SplineComponent.GetRotationAtDistanceAlongSpline` (`self.Spline`) (`self.Distance`) "World")) false false)
  (`SceneComponent.K2_AddWorldRotation` (`self.SkeletalMesh`) (struct :`Yaw` -90.0) false false))

(fn `UserConstructionScript`)