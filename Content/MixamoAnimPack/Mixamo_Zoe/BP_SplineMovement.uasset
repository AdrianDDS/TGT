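; BP_SplineMovement is an actor that moves a skeletal mesh along its spline.
; On BeginPlay a Progression timeline drives an alpha that, scaled by spline length, places the mesh at that distance's world location and rotation.
; Each update also applies a -90 yaw correction and prints a debug string.
; Velocity-reading nodes are left unconnected, noted as not returning the character's speed.
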(event `self.ReceiveBeginPlay`
  (bind _spline (`self.Spline`))
  (bind (_direction _progression_alpha) (`Timeline|Progression` :!via `PlayFromStart`)
    (:`Update`
      (bind _returnvalue (* (`SplineComponent.GetSplineLength` _spline) _progression_alpha))
      (`SceneComponent.K2_SetWorldTransform` (`self.SkeletalMesh`) (`KismetMathLibrary.MakeTransform` (`SplineComponent.GetLocationAtDistanceAlongSpline` _spline _returnvalue "World") (`SplineComponent.GetRotationAtDistanceAlongSpline` (`self.Spline`) _returnvalue "World")) false false)
      (`SceneComponent.K2_AddWorldRotation` (`self.SkeletalMesh`) (struct :`Yaw` -90.0) false false)
      (`KismetSystemLibrary.PrintString` "Hello"))))

(fn `UserConstructionScript`)