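; Goober character Blueprint that sets facial expressions by choosing mouth, eye and eyebrow textures from per-part index numbers.
; The construction script maps each number to a texture and applies it through dynamic material instances on separate SKGoober material slots.
; Tick repeats this through per-part selection macros, creating new dynamic material instances every frame.
; Many eyebrow indices and some left-eye indices resolve to an empty texture.
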(event `self.ReceiveTick`
  (params (DeltaSeconds :type "Float (single-precision)"))
  (bind _returnvalue (`PrimitiveComponent.CreateDynamicMaterialInstance` (`self.SK_Goober`) 5 "/Game/Characters/Goober/Materials/M_Mouth.M_Mouth" "None"))
  (switch `int` (`self.MouthNumber`)
    (:`Default`
      (set `self.Mouth Texture` "/Game/Characters/Faces/T_Mouth01.T_Mouth01" :!label _label))
    (:`0`
      (set `self.Mouth Texture` "/Game/Characters/Faces/T_Empty.T_Empty"))
    (:`1`
      (goto _label))
    (:`2`
      (set `self.Mouth Texture` "/Game/Characters/Faces/T_Mouth02.T_Mouth02"))
    (:`3`
      (set `self.Mouth Texture` "/Game/Characters/Faces/T_Mouth03.T_Mouth03"))
    (:`4`
      (set `self.Mouth Texture` "/Game/Characters/Faces/T_Mouth04.T_Mouth04"))
    (:`5`
      (set `self.Mouth Texture` "/Game/Characters/Faces/T_Mouth05.T_Mouth05"))
    (:`6`
      (set `self.Mouth Texture` "/Game/Characters/Faces/T_Mouth06.T_Mouth06"))
    (:`7`
      (set `self.Mouth Texture` "/Game/Characters/Faces/T_Mouth07.T_Mouth07"))
    (:`8`
      (set `self.Mouth Texture` "/Game/Characters/Faces/T_Mouth08.T_Mouth08"))
    (:`9`
      (set `self.Mouth Texture` "/Game/Characters/Faces/T_Mouth09.T_Mouth09"))
    (:`10`
      (set `self.Mouth Texture` "/Game/Characters/Faces/T_Mouth10.T_Mouth10"))
    (:`11`
      (set `self.Mouth Texture` "/Game/Characters/Faces/T_Mouth11.T_Mouth11"))
    (:`12`
      (set `self.Mouth Texture` "/Game/Characters/Faces/T_Mouth12.T_Mouth12"))
    (:`13`
      (set `self.Mouth Texture` "/Game/Characters/Faces/T_Mouth013.T_Mouth013"))
    (:`14`
      (set `self.Mouth Texture` "/Game/Characters/Faces/T_Mouth14.T_Mouth14"))
    (:`15`
      (set `self.Mouth Texture` "/Game/Characters/Faces/T_Mouth15.T_Mouth15"))
    (:`16`
      (set `self.Mouth Texture` "/Game/Characters/Faces/T_Mouth16.T_Mouth16"))
    (:`17`
      (set `self.Mouth Texture` "/Game/Characters/Faces/T_Mouth17.T_Mouth17"))
    (:`18`
      (set `self.Mouth Texture` "/Game/Characters/Faces/T_Mouth18.T_Mouth18"))
    (:`19`
      (set `self.Mouth Texture` "/Game/Characters/Faces/T_Mouth19.T_Mouth19"))
    (:`20`
      (set `self.Mouth Texture` "/Game/Characters/Faces/T_Mouth20.T_Mouth20"))
    (:`21`
      (set `self.Mouth Texture` "/Game/Characters/Faces/T_Mouth21.T_Mouth21"))
    (:`22`
      (set `self.Mouth Texture` "/Game/Characters/Faces/T_Mouth22.T_Mouth22"))
    (:`23`
      (set `self.Mouth Texture` "/Game/Characters/Faces/T_Mouth23.T_Mouth23"))
    (:`24`
      (set `self.Mouth Texture` "/Game/Characters/Faces/T_Mouth24.T_Mouth24"))
    (:`25`
      (set `self.Mouth Texture` "/Game/Characters/Faces/T_Mouth25.T_Mouth25"))
    (:`26`
      (set `self.Mouth Texture` "/Game/Characters/Faces/T_Mouth26.T_Mouth26"))
    (:`27`
      (set `self.Mouth Texture` "/Game/Characters/Faces/T_Mouth27.T_Mouth27"))
    (:`28`
      (set `self.Mouth Texture` "/Game/Characters/Faces/T_Mouth28.T_Mouth28")))
  (`MaterialInstanceDynamic.SetTextureParameterValue` _returnvalue "Mouth Texture" (`self.Mouth Texture`)) ; Cambia la textura de la boca
  (bind _returnvalue_2 (`PrimitiveComponent.CreateDynamicMaterialInstance` (`self.SK_Goober`) 3 "/Game/Characters/Goober/Materials/M_Eye_R.M_Eye_R" "None"))
  (switch `int` (`self.RightEyeNumber`)
    (:`Default`
      (set `self.Right Eye Texture` "/Game/Characters/Faces/T_Eye01_R.T_Eye01_R" :!label _label_2))
    (:`0`
      (set `self.Right Eye Texture` "/Game/Characters/Faces/T_Empty.T_Empty"))
    (:`1`
      (goto _label_2))
    (:`2`
      (set `self.Right Eye Texture` "/Game/Characters/Faces/T_Eye02_R.T_Eye02_R"))
    (:`3`
      (set `self.Right Eye Texture` "/Game/Characters/Faces/T_Eye03_R.T_Eye03_R"))
    (:`4`
      (set `self.Right Eye Texture` "/Game/Characters/Faces/T_Eye04_R.T_Eye04_R"))
    (:`5`
      (set `self.Right Eye Texture` "/Game/Characters/Faces/T_Eye05_R.T_Eye05_R"))
    (:`6`
      (set `self.Right Eye Texture` "/Game/Characters/Faces/T_Eye06_R.T_Eye06_R"))
    (:`7`
      (set `self.Right Eye Texture` "/Game/Characters/Faces/T_Eye07_R.T_Eye07_R"))
    (:`8`
      (set `self.Right Eye Texture` "/Game/Characters/Faces/T_Eye08_R.T_Eye08_R"))
    (:`9`
      (set `self.Right Eye Texture` "/Game/Characters/Faces/T_Eye09_R.T_Eye09_R"))
    (:`10`
      (set `self.Right Eye Texture` "/Game/Characters/Faces/T_Eye10_R.T_Eye10_R"))
    (:`11`
      (set `self.Right Eye Texture` "/Game/Characters/Faces/T_Eye11_R.T_Eye11_R"))
    (:`12`
      (set `self.Right Eye Texture` "/Game/Characters/Faces/T_Eye12_R.T_Eye12_R"))
    (:`13`
      (set `self.Right Eye Texture` "/Game/Characters/Faces/T_Eye13_R.T_Eye13_R")))
  (`MaterialInstanceDynamic.SetTextureParameterValue` _returnvalue_2 "Eye_R Texture" (`self.Right Eye Texture`)) ; Cambia la textura del ojo derecho
  (bind _returnvalue_3 (`PrimitiveComponent.CreateDynamicMaterialInstance` (`self.SK_Goober`) 4 "/Game/Characters/Goober/Materials/M_Eye_L.M_Eye_L" "None"))
  (switch `int` (`self.LeftEyeNumber`)
    (:`Default`
      (set `self.Left Eye Texture` "/Game/Characters/Faces/T_Eye01_L.T_Eye01_L" :!label _label_3))
    (:`0`
      (set `self.Left Eye Texture` "/Game/Characters/Faces/T_Empty.T_Empty"))
    (:`1`
      (goto _label_3))
    (:`2`
      (set `self.Left Eye Texture` "/Game/Characters/Faces/T_Eye02_L.T_Eye02_L"))
    (:`3`
      (set `self.Left Eye Texture` "/Game/Characters/Faces/T_Eye03_L.T_Eye03_L"))
    (:`4`
      (set `self.Left Eye Texture` "/Game/Characters/Faces/T_Eye04_L.T_Eye04_L"))
    (:`5`
      (set `self.Left Eye Texture` "/Game/Characters/Faces/T_Eye05_L.T_Eye05_L"))
    (:`6`
      (set `self.Left Eye Texture` "/Game/Characters/Faces/T_Empty.T_Empty"))
    (:`7`
      (set `self.Left Eye Texture` "/Game/Characters/Faces/T_Eye07_L.T_Eye07_L"))
    (:`8`
      (set `self.Left Eye Texture` "/Game/Characters/Faces/T_Eye08_L.T_Eye08_L"))
    (:`9`
      (set `self.Left Eye Texture` "/Game/Characters/Faces/T_Empty.T_Empty"))
    (:`10`
      (set `self.Left Eye Texture` "/Game/Characters/Faces/T_Empty.T_Empty"))
    (:`11`
      (set `self.Left Eye Texture` "/Game/Characters/Faces/T_Eye11_L.T_Eye11_L"))
    (:`12`
      (set `self.Left Eye Texture` "/Game/Characters/Faces/T_Eye12_L.T_Eye12_L"))
    (:`13`
      (set `self.Left Eye Texture` "/Game/Characters/Faces/T_Eyebrow13_L.T_Eyebrow13_L")))
  (`MaterialInstanceDynamic.SetTextureParameterValue` _returnvalue_3 "Eye_L Texture" (`self.Left Eye Texture`)) ; Cambia la textura del ojo izquierdo
  (bind _returnvalue_4 (`PrimitiveComponent.CreateDynamicMaterialInstance` (`self.SK_Goober`) 1 "/Game/Characters/Goober/Materials/M_Eyebrow_R.M_Eyebrow_R" "None"))
  (switch `int` (`self.RightEyebrowNumber`)
    (:`Default`
      (set `self.Right Eyebrow Texture` "/Game/Characters/Faces/T_Empty.T_Empty" :!label _label_4))
    (:`0`
      (goto _label_4))
    (:`1`
      (goto _label_4))
    (:`2`
      (goto _label_4))
    (:`3`
      (goto _label_4))
    (:`4`
      (goto _label_4))
    (:`5`
      (goto _label_4))
    (:`6`
      (goto _label_4))
    (:`7`
      (goto _label_4))
    (:`8`
      (goto _label_4))
    (:`9`
      (goto _label_4))
    (:`10`
      (goto _label_4))
    (:`11`
      (goto _label_4))
    (:`12`
      (set `self.Right Eyebrow Texture` "/Game/Characters/Faces/T_Eyebrow12_R.T_Eyebrow12_R"))
    (:`13`
      (set `self.Right Eyebrow Texture` "/Game/Characters/Faces/T_Eyebrow13_R.T_Eyebrow13_R")))
  (`MaterialInstanceDynamic.SetTextureParameterValue` _returnvalue_4 "Eyebrow_R Texture" (`self.Right Eyebrow Texture`)) ; Cambia la textura de la ceja derecha
  (bind _returnvalue_5 (`PrimitiveComponent.CreateDynamicMaterialInstance` (`self.SK_Goober`) 2 "/Game/Characters/Goober/Materials/M_Eyebrow_L.M_Eyebrow_L" "None"))
  (switch `int` (`self.LeftEyebrowNumber`)
    (:`Default`
      (set `self.Left Eyebrow Texture` "/Game/Characters/Faces/T_Eyebrow12_L.T_Eyebrow12_L" :!label _label_5))
    (:`0`
      (set `self.Left Eyebrow Texture` "/Game/Characters/Faces/T_Empty.T_Empty" :!label _label_6))
    (:`1`
      (goto _label_6))
    (:`2`
      (goto _label_6))
    (:`3`
      (goto _label_6))
    (:`4`
      (goto _label_6))
    (:`5`
      (goto _label_6))
    (:`6`
      (goto _label_6))
    (:`7`
      (goto _label_6))
    (:`8`
      (goto _label_6))
    (:`9`
      (goto _label_6))
    (:`10`
      (goto _label_6))
    (:`11`
      (goto _label_6))
    (:`12`
      (goto _label_5))
    (:`13`
      (set `self.Left Eyebrow Texture` "/Game/Characters/Faces/T_Eyebrow13_L.T_Eyebrow13_L")))
  (`MaterialInstanceDynamic.SetTextureParameterValue` _returnvalue_5 "Eyebrow_L Texture" (`self.Left Eyebrow Texture`)) ; Cambia la textura de la ceja izquierda
)

(fn `UserConstructionScript`
  (bind _returnvalue (`PrimitiveComponent.CreateDynamicMaterialInstance` (`self.SK_Goober`) 5 "/Game/Characters/Goober/Materials/M_Mouth.M_Mouth" "None")) ; Set Mouth textures
  (switch `int` (`self.MouthNumber`)
    (:`Default`
      (set `self.Mouth Texture` "/Game/Characters/Faces/T_Mouth01.T_Mouth01" :!label _label))
    (:`0`
      (set `self.Mouth Texture` "/Game/Characters/Faces/T_Empty.T_Empty"))
    (:`1`
      (goto _label))
    (:`2`
      (set `self.Mouth Texture` "/Game/Characters/Faces/T_Mouth02.T_Mouth02"))
    (:`3`
      (set `self.Mouth Texture` "/Game/Characters/Faces/T_Mouth03.T_Mouth03"))
    (:`4`
      (set `self.Mouth Texture` "/Game/Characters/Faces/T_Mouth04.T_Mouth04"))
    (:`5`
      (set `self.Mouth Texture` "/Game/Characters/Faces/T_Mouth05.T_Mouth05"))
    (:`6`
      (set `self.Mouth Texture` "/Game/Characters/Faces/T_Mouth06.T_Mouth06"))
    (:`7`
      (set `self.Mouth Texture` "/Game/Characters/Faces/T_Mouth07.T_Mouth07"))
    (:`8`
      (set `self.Mouth Texture` "/Game/Characters/Faces/T_Mouth08.T_Mouth08"))
    (:`9`
      (set `self.Mouth Texture` "/Game/Characters/Faces/T_Mouth09.T_Mouth09"))
    (:`10`
      (set `self.Mouth Texture` "/Game/Characters/Faces/T_Mouth10.T_Mouth10"))
    (:`11`
      (set `self.Mouth Texture` "/Game/Characters/Faces/T_Mouth11.T_Mouth11"))
    (:`12`
      (set `self.Mouth Texture` "/Game/Characters/Faces/T_Mouth12.T_Mouth12"))
    (:`13`
      (set `self.Mouth Texture` "/Game/Characters/Faces/T_Mouth013.T_Mouth013"))
    (:`14`
      (set `self.Mouth Texture` "/Game/Characters/Faces/T_Mouth14.T_Mouth14"))
    (:`15`
      (set `self.Mouth Texture` "/Game/Characters/Faces/T_Mouth15.T_Mouth15"))
    (:`16`
      (set `self.Mouth Texture` "/Game/Characters/Faces/T_Mouth16.T_Mouth16"))
    (:`17`
      (set `self.Mouth Texture` "/Game/Characters/Faces/T_Mouth17.T_Mouth17"))
    (:`18`
      (set `self.Mouth Texture` "/Game/Characters/Faces/T_Mouth18.T_Mouth18"))
    (:`19`
      (set `self.Mouth Texture` "/Game/Characters/Faces/T_Mouth19.T_Mouth19"))
    (:`20`
      (set `self.Mouth Texture` "/Game/Characters/Faces/T_Mouth20.T_Mouth20"))
    (:`21`
      (set `self.Mouth Texture` "/Game/Characters/Faces/T_Mouth21.T_Mouth21"))
    (:`22`
      (set `self.Mouth Texture` "/Game/Characters/Faces/T_Mouth22.T_Mouth22"))
    (:`23`
      (set `self.Mouth Texture` "/Game/Characters/Faces/T_Mouth23.T_Mouth23"))
    (:`24`
      (set `self.Mouth Texture` "/Game/Characters/Faces/T_Mouth24.T_Mouth24"))
    (:`25`
      (set `self.Mouth Texture` "/Game/Characters/Faces/T_Mouth25.T_Mouth25"))
    (:`26`
      (set `self.Mouth Texture` "/Game/Characters/Faces/T_Mouth26.T_Mouth26"))
    (:`27`
      (set `self.Mouth Texture` "/Game/Characters/Faces/T_Mouth27.T_Mouth27"))
    (:`28`
      (set `self.Mouth Texture` "/Game/Characters/Faces/T_Mouth28.T_Mouth28")))
  (`MaterialInstanceDynamic.SetTextureParameterValue` _returnvalue "Mouth Texture" (`self.Mouth Texture`))
  (bind _returnvalue_2 (`PrimitiveComponent.CreateDynamicMaterialInstance` (`self.SK_Goober`) 3 "/Game/Characters/Goober/Materials/M_Eye_R.M_Eye_R" "None")) ; Set Right Eye Textures
  (switch `int` (`self.RightEyeNumber`)
    (:`Default`
      (set `self.Right Eye Texture` "/Game/Characters/Faces/T_Eye01_R.T_Eye01_R" :!label _label_2))
    (:`0`
      (set `self.Right Eye Texture` "/Game/Characters/Faces/T_Empty.T_Empty"))
    (:`1`
      (goto _label_2))
    (:`2`
      (set `self.Right Eye Texture` "/Game/Characters/Faces/T_Eye02_R.T_Eye02_R"))
    (:`3`
      (set `self.Right Eye Texture` "/Game/Characters/Faces/T_Eye03_R.T_Eye03_R"))
    (:`4`
      (set `self.Right Eye Texture` "/Game/Characters/Faces/T_Eye04_R.T_Eye04_R"))
    (:`5`
      (set `self.Right Eye Texture` "/Game/Characters/Faces/T_Eye05_R.T_Eye05_R"))
    (:`6`
      (set `self.Right Eye Texture` "/Game/Characters/Faces/T_Eye06_R.T_Eye06_R"))
    (:`7`
      (set `self.Right Eye Texture` "/Game/Characters/Faces/T_Eye07_R.T_Eye07_R"))
    (:`8`
      (set `self.Right Eye Texture` "/Game/Characters/Faces/T_Eye08_R.T_Eye08_R"))
    (:`9`
      (set `self.Right Eye Texture` "/Game/Characters/Faces/T_Eye09_R.T_Eye09_R"))
    (:`10`
      (set `self.Right Eye Texture` "/Game/Characters/Faces/T_Eye10_R.T_Eye10_R"))
    (:`11`
      (set `self.Right Eye Texture` "/Game/Characters/Faces/T_Eye11_R.T_Eye11_R"))
    (:`12`
      (set `self.Right Eye Texture` "/Game/Characters/Faces/T_Eye12_R.T_Eye12_R"))
    (:`13`
      (set `self.Right Eye Texture` "/Game/Characters/Faces/T_Eye13_R.T_Eye13_R")))
  (`MaterialInstanceDynamic.SetTextureParameterValue` _returnvalue_2 "Eye_R Texture" (`self.Right Eye Texture`))
  (bind _returnvalue_3 (`PrimitiveComponent.CreateDynamicMaterialInstance` (`self.SK_Goober`) 4 "/Game/Characters/Goober/Materials/M_Eye_L.M_Eye_L" "None")) ; Set Left Eye Textures
  (switch `int` (`self.LeftEyeNumber`)
    (:`Default`
      (set `self.Left Eye Texture` "/Game/Characters/Faces/T_Eye01_L.T_Eye01_L" :!label _label_3))
    (:`0`
      (set `self.Left Eye Texture` "/Game/Characters/Faces/T_Empty.T_Empty"))
    (:`1`
      (goto _label_3))
    (:`2`
      (set `self.Left Eye Texture` "/Game/Characters/Faces/T_Eye02_L.T_Eye02_L"))
    (:`3`
      (set `self.Left Eye Texture` "/Game/Characters/Faces/T_Eye03_L.T_Eye03_L"))
    (:`4`
      (set `self.Left Eye Texture` "/Game/Characters/Faces/T_Eye04_L.T_Eye04_L"))
    (:`5`
      (set `self.Left Eye Texture` "/Game/Characters/Faces/T_Eye05_L.T_Eye05_L"))
    (:`6`
      (set `self.Left Eye Texture` "/Game/Characters/Faces/T_Empty.T_Empty"))
    (:`7`
      (set `self.Left Eye Texture` "/Game/Characters/Faces/T_Eye07_L.T_Eye07_L"))
    (:`8`
      (set `self.Left Eye Texture` "/Game/Characters/Faces/T_Eye08_L.T_Eye08_L"))
    (:`9`
      (set `self.Left Eye Texture` "/Game/Characters/Faces/T_Empty.T_Empty"))
    (:`10`
      (set `self.Left Eye Texture` "/Game/Characters/Faces/T_Empty.T_Empty"))
    (:`11`
      (set `self.Left Eye Texture` "/Game/Characters/Faces/T_Eye11_L.T_Eye11_L"))
    (:`12`
      (set `self.Left Eye Texture` "/Game/Characters/Faces/T_Eye12_L.T_Eye12_L"))
    (:`13`
      (set `self.Left Eye Texture` "/Game/Characters/Faces/T_Eyebrow13_L.T_Eyebrow13_L")))
  (`MaterialInstanceDynamic.SetTextureParameterValue` _returnvalue_3 "Eye_L Texture" (`self.Left Eye Texture`))
  (bind _returnvalue_4 (`PrimitiveComponent.CreateDynamicMaterialInstance` (`self.SK_Goober`) 1 "/Game/Characters/Goober/Materials/M_Eyebrow_R.M_Eyebrow_R" "None")) ; Set Right Eyebrow Textures
  (switch `int` (`self.RightEyebrowNumber`)
    (:`Default`
      (set `self.Right Eyebrow Texture` "/Game/Characters/Faces/T_Empty.T_Empty" :!label _label_4))
    (:`0`
      (goto _label_4))
    (:`1`
      (goto _label_4))
    (:`2`
      (goto _label_4))
    (:`3`
      (goto _label_4))
    (:`4`
      (goto _label_4))
    (:`5`
      (goto _label_4))
    (:`6`
      (goto _label_4))
    (:`7`
      (goto _label_4))
    (:`8`
      (goto _label_4))
    (:`9`
      (goto _label_4))
    (:`10`
      (goto _label_4))
    (:`11`
      (goto _label_4))
    (:`12`
      (set `self.Right Eyebrow Texture` "/Game/Characters/Faces/T_Eyebrow12_R.T_Eyebrow12_R"))
    (:`13`
      (set `self.Right Eyebrow Texture` "/Game/Characters/Faces/T_Eyebrow13_R.T_Eyebrow13_R")))
  (`MaterialInstanceDynamic.SetTextureParameterValue` _returnvalue_4 "Eyebrow_R Texture" (`self.Right Eyebrow Texture`))
  (bind _returnvalue_5 (`PrimitiveComponent.CreateDynamicMaterialInstance` (`self.SK_Goober`) 2 "/Game/Characters/Goober/Materials/M_Eyebrow_L.M_Eyebrow_L" "None")) ; Set Left Eyebrow Textures
  (switch `int` (`self.LeftEyebrowNumber`)
    (:`Default`
      (set `self.Left Eyebrow Texture` "/Game/Characters/Faces/T_Eyebrow12_L.T_Eyebrow12_L" :!label _label_5))
    (:`0`
      (set `self.Left Eyebrow Texture` "/Game/Characters/Faces/T_Empty.T_Empty" :!label _label_6))
    (:`1`
      (goto _label_6))
    (:`2`
      (goto _label_6))
    (:`3`
      (goto _label_6))
    (:`4`
      (goto _label_6))
    (:`5`
      (goto _label_6))
    (:`6`
      (goto _label_6))
    (:`7`
      (goto _label_6))
    (:`8`
      (goto _label_6))
    (:`9`
      (goto _label_6))
    (:`10`
      (goto _label_6))
    (:`11`
      (goto _label_6))
    (:`12`
      (goto _label_5))
    (:`13`
      (set `self.Left Eyebrow Texture` "/Game/Characters/Faces/T_Eyebrow13_L.T_Eyebrow13_L")))
  (`MaterialInstanceDynamic.SetTextureParameterValue` _returnvalue_5 "Eyebrow_L Texture" (`self.Left Eyebrow Texture`)))