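; Goober character Blueprint that computes aim angles toward a target actor.
; A looping timer started on BeginPlay runs UpdateAim 18 times a second instead of using Tick, though the Spanish comment says 12.
; UpdateAim sets the target to the player pawn when LootAtPlayer is on, then stores look-at Pitch and Yaw from a point raised above SKGoober.
; The target is not checked for validity.
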(event `self.ReceiveBeginPlay`
  (`KismetSystemLibrary.K2_SetTimerDelegate` (delegate `Update Aim`) (/ 1.0 18.0) true) ; La orientación del personaje se actualiza 12 veces/segundo
)

(event `Update Aim`
  (if (`self.LootAtPlayer`)
    (bind _output_get (set `self.Target Actor` (`GameplayStatics.GetPlayerPawn` 0))))
  (bind (_returnvalue_roll _returnvalue_pitch _returnvalue_yaw) (`KismetMathLibrary.BreakRotator` (`KismetMathLibrary.FindLookAtRotation` (+ (`SceneComponent.K2_GetComponentLocation` (`self.SK_Goober`)) (0.0 0.0 150.0)) (`SceneComponent.K2_GetComponentLocation` (`Actor.RootComponent` _output_get)))))
  (set `self.Pitch` _returnvalue_pitch)
  (set `self.Yaw` _returnvalue_yaw))

(fn `UserConstructionScript`)