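; Goober actor that moves its SKGoober component along a spline.
; Each Tick advances Distance by Speed, sets the component's world transform from that spline point, then adds a fixed 90-degree rotation offset.
; It also calculates velocity using a newly made position history each frame, prints it, and stores a scaled copy in ActualSpeed.
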(event `self.ReceiveBeginPlay`)

(event `self.ReceiveTick`
  (params (DeltaSeconds :type "Float (single-precision)"))
  (bind _returnvalue (`SplineComponent.GetLocationAtDistanceAlongSpline` (`self.Spline`) (`self.Distance`) "World"))
  (set `self.Distance` (+ (* DeltaSeconds (`self.Speed`)) (`self.Distance`)))
  (`SceneComponent.K2_SetWorldTransform` (`self.SK_Goober`) (`KismetMathLibrary.MakeTransform` _returnvalue (`SplineComponent.GetRotationAtDistanceAlongSpline` (`self.Spline`) (`self.Distance`) "World")) false false)
  (`SceneComponent.K2_AddWorldRotation` (`self.SK_Goober`) (struct :`Yaw` 90.0) false false)
  ;[1 1 1] Casi
  (bind _returnvalue_2 (`KismetAnimationLibrary.K2_CalculateVelocityFromPositionHistory` DeltaSeconds _returnvalue (make `PositionHistory`) 16 "0.f" 256.0))
  (`KismetSystemLibrary.PrintString` (`KismetStringLibrary.Conv_DoubleToString` _returnvalue_2))
  (set `self.ActualSpeed` (* _returnvalue_2 300.0)))

(fn `UserConstructionScript`)